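; BP_Nexus is the Nexus actor of the tower defense game, a damageable objective whose destruction ends the game.
; Its AnyDamage event subtracts incoming damage from NexusHp unless the Godmode flag is set.
; When health reaches zero or below, it hides its Cube component, adds a BP_GameOver widget to the viewport and pauses the game.
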(event Game|Damage|EventAnyDamage
  (params (Damage :type Float%20%28single-precision%29) (DamageType :type Damage%20Type%20Object%20Reference) (InstigatedBy :type Controller%20Object%20Reference) (DamageCauser :type Actor%20Object%20Reference))
  (if (not (Variables|Default|Getgodmode))
    (bind _output_get (Variables|Default|Setnexus_Hp (- (Variables|Default|Getnexus_Hp) Damage)))
    (if (<= _output_get 0.0)
      (Rendering|SetVisibility (Variables|Default|GetCube) false false)
      (bind _returnvalue (UserInterface|CreateWidget "/Game/ActiveTowerDefense/Blueprints/UI/BP_gameOver.BP_GameOver_C"))
      (UserInterface|Viewport|AddtoViewport _returnvalue 0)
      (Game|SetGamePaused true))))

(fn ConstructionScript)