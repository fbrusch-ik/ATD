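; BP_Ghost is a ghost actor in the tower defense game, configured by its elemental Type.
; The construction script loads table data for that Type and hands the mesh to its selectable component.
; On BeginPlay it sets the nameplate's elemental icon, then waits a random delay of up to two seconds before looping the idle animation, so ghosts animate out of sync.
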(event EventBeginPlay
  (bind _asbp_elemental_icon (Utilities|Casting|CastToBP_ElementalIcon (UserInterface|GetUserWidgetObject (Variables|Default|GetNameplate))))
  (Default|SetIcon _asbp_elemental_icon (Variables|Default|GetType))
  (Utilities|FlowControl|Delay (* (Math|Random|RandomFloat) 2.0))
  (Components|Animation|PlayAnimation (Variables|Character|GetMesh) "/Game/ActiveTowerDefense/Blueprints/Ghosts/A_Ghost_Idle.A_Ghost_Idle" true))

(event Collision|EventActorBeginOverlap
  (params (OtherActor :type Actor%20Object%20Reference)))

(event EventTick
  (params (DeltaSeconds :type Float%20%28single-precision%29)))

(fn ConstructionScript
  (bind _newparam (CallFunction|GetGhostData (Variables|Default|GetType)))
  (Variables|Default|SetTableData _newparam)
  (Variables|/Game/ActiveTowerDefense/Blueprints/Components/BP_Selectable.BP_Selectable_C|SetMesh (Variables|Default|GetBP_Selectable) (Variables|Character|GetMesh)))