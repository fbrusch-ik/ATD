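; Tower defense manager that doubles as the damageable Nexus, alternating Build and Attack phases and pausing on Game Over when Nexus HP runs out.
; A one-second looping timer counts down each phase, with both reset to AttackTimeMax and each attack advancing the Section.
; During attacks it scans the WaveData table for rows matching Section and elapsed time, spawning that ball enemy type at the slot-indexed BP_Spawn actor.
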(event Custom|Tick
  (switch Utilities|FlowControl|Switch|SwitchonGamePhase (Variables|Default|GetcurrentPhase)
    (:NewEnumerator0
      (CallFunction|BuildTick))
    (:NewEnumerator1
      (CallFunction|AttackTick))))

(event EventBeginPlay
  (Utilities|Time|SetTimerbyEvent (delegate Custom|Tick) 1.0 true))

(event Game|Damage|EventAnyDamage
  (params (Damage :type Float%20%28single-precision%29) (DamageType :type Damage%20Type%20Object%20Reference) (InstigatedBy :type Controller%20Object%20Reference) (DamageCauser :type Actor%20Object%20Reference))
  (if (not (Variables|Default|Getgodmode))
    (bind _output_get (Variables|Default|Setnexus_Hp (- (Variables|Default|Getnexus_Hp) Damage)))
    (if (<= _output_get 0.0)
      (Rendering|SetVisibility (Variables|Default|GetCube) false false)
      (bind _returnvalue (UserInterface|CreateWidget "/Game/ActiveTowerDefense/Blueprints/UI/BP_gameOver.BP_GameOver_C"))
      (UserInterface|Viewport|AddtoViewport _returnvalue 0)
      (Game|SetGamePaused true))))

(fn ConstructionScript)

(fn Spawn
  (params (What :type WaveTypes%20Enum :default "NewEnumerator0") (Slot :type Integer))
  (bind _outactors (Actor|GetAllActorsOfClass "/Game/ActiveTowerDefense/Blueprints/BP_Spawn.BP_Spawn_C"))
  (switch Utilities|FlowControl|Switch|SwitchonWaveTypes What
    (:NewEnumerator0
      (Variables|Default|SettoSpawn "/Game/ActiveTowerDefense/Blueprints/BP_GreenBall.BP_GreenBall_C"))
    (:NewEnumerator1
      (Variables|Default|SettoSpawn "/Game/ActiveTowerDefense/Blueprints/BP_RedBall.BP_RedBall_C"))
    (:NewEnumerator2
      (Variables|Default|SettoSpawn "/Game/ActiveTowerDefense/Blueprints/BP_BlueBall.BP_BlueBall_C"))
    (:NewEnumerator5
      (Variables|Default|SettoSpawn "/Game/ActiveTowerDefense/Blueprints/BP_Enemy.BP_Enemy_C")))
  (AI|SpawnAIFromClass (Variables|Default|GettoSpawn) 0 (Transformation|GetActorLocation (Utilities|Array|Get(acopy) _outactors (+ Slot -1))) "0, 0, 0" false 0))

(fn BuildTick
  (bind _result (Math|Float|DecrementFloat (Variables|Default|GetphaseTimeRemaining))
    (:%20%20
      (if (<= _result 0.0)
        (CallFunction|StartAttack)))))

(fn AttackTick
  (bind _result (Math|Float|DecrementFloat (Variables|Default|GetphaseTimeRemaining))
    (:%20%20
      (if (<= _result 0.0)
        (CallFunction|StartBuild)
        (else
          (bind _outrownames (DataTable|GetDataTableRowNames "/Game/ActiveTowerDefense/Data/WaveData.WaveData"))
          (for _array_element _outrownames
            (bind _returnvalue (Utilities|GetDataTableRow "/Game/ActiveTowerDefense/Data/WaveData.WaveData" _array_element)
              (:then
                (if (and (== (.section _returnvalue) (Variables|Default|GetSection)) (== (.time _returnvalue) (- (Variables|Default|GetAttackTimeMax) (Variables|Default|GetphaseTimeRemaining))))
                  (CallFunction|Spawn (.type _returnvalue) (.slot _returnvalue)))))))))))

(fn StartAttack
  (Variables|Default|SetphaseTimeRemaining (Variables|Default|GetAttackTimeMax))
  (Math|Integer|IncrementInt (Variables|Default|GetSection)
    (:%20%20
      (Variables|Default|SetcurrentPhase "NewEnumerator1"))))

(fn StartBuild
  (Variables|Default|SetphaseTimeRemaining (Variables|Default|GetAttackTimeMax))
  (Variables|Default|SetcurrentPhase "NewEnumerator0"))