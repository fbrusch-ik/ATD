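; BP_Enemy is a tower defense enemy that travels to the BP_Gamestate actor, damages it on arrival and destroys itself.
; After a short delay on BeginPlay, AI MoveTo drives it toward that actor.
; Incoming damage lowers its health and calls EnemyDefeated at zero, or on any hit while the gamestate's Godmode is on.
; Separate functions destroy the actor and set its green, red or blue element material from EnemyType.
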(event EventBeginPlay
  (Utilities|FlowControl|Delay 0.2)
  (bind _returnvalue (Actor|GetActorOfClass "/Game/ActiveTowerDefense/Blueprints/BP_Gamestate.BP_Gamestate_C"))
  (AI|AIMoveTo self "0, 0, 0" _returnvalue 5.0 false
    (:OnSuccess
      (Game|Damage|ApplyDamage _returnvalue (Variables|Default|Getenemy_damage) 0 0)
      (Actor|DestroyActor))))

(event Game|Damage|EventAnyDamage
  (params (Damage :type Float%20%28single-precision%29) (DamageType :type Damage%20Type%20Object%20Reference) (InstigatedBy :type Controller%20Object%20Reference) (DamageCauser :type Actor%20Object%20Reference))
  (bind _output_get (Variables|Default|Setenemy_hp (- (Variables|Default|Getenemy_hp) Damage)))
  (if (<= _output_get 0.0)
    (CallFunction|EnemyDefeated self :!label _label)
    (else
      (bind _returnvalue (Actor|GetActorOfClass "/Game/ActiveTowerDefense/Blueprints/BP_Gamestate.BP_Gamestate_C"))
      (if (Variables|/Game/ActiveTowerDefense/Blueprints/BP_Gamestate.BP_Gamestate_C|Getgodmode _returnvalue)
        (goto _label)))))

(fn ConstructionScript)

(fn DefeatEnemy
  (Actor|DestroyActor))

(fn UpdateMaterial
  (switch Utilities|FlowControl|Switch|SwitchonE_Elements (Variables|Default|Getenemy_type)
    (:NewEnumerator0
      (LocalVariables|Setmat "/Game/ActiveTowerDefense/Materials/M_Element_Green.M_Element_Green"))
    (:NewEnumerator1
      (LocalVariables|Setmat "/Game/ActiveTowerDefense/Materials/M_Element_Red.M_Element_Red"))
    (:NewEnumerator2
      (LocalVariables|Setmat "/Game/ActiveTowerDefense/Materials/M_Element_Blue.M_Element_Blue")))
  (Rendering|Material|SetMaterial (Variables|Default|Getenemy) 0 (LocalVariables|Getmat)))