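; Normal enemy for the tower defense game that splits into smaller-health copies of itself when defeated.
; Defeat spawns four AI copies at random navigable points nearby, then destroys the original.
; Each copy is flagged as Child, gets reduced HP and a set walk speed, inherits the Affix and refreshes its material.
; The Child flag stops recursion, so defeated copies are simply destroyed.
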(event EventBeginPlay
  (|CallParentFunction) ; This node is disabled and will not be called.\nDrag off pins to build functionality.
)

(event Collision|EventActorBeginOverlap
  (params (OtherActor :type Actor%20Object%20Reference)))

(event EventTick
  (params (DeltaSeconds :type Float%20%28single-precision%29)))

(fn ConstructionScript
  (|CallParentFunction))

(fn Defeat
  (if (Variables|Default|Getchild)
    (Actor|DestroyActor)
    (else
      (for _index (range 1 4)
        (bind _randomlocation (Class|NavigationSystemV1|GetRandomLocationinNavigableRadius (Transformation|GetActorLocation) 3e+02 0 0))
        (bind _returnvalue (AI|SpawnAIFromClass "BP_Enemy_Normal_C" 0 _randomlocation "0, 0, 0" false 0))
        (bind _asbp_split (Utilities|Casting|CastToBP_Enemy_Normal _returnvalue))
        (Variables|BP_Enemy_Normal_C|Setchild _asbp_split true)
        (Variables|/Game/ActiveTowerDefense/Blueprints/BP_Enemy.BP_Enemy_C|SetHP _asbp_split (/ (Variables|/Game/ActiveTowerDefense/Blueprints/BP_Enemy.BP_Enemy_C|GetHP _asbp_split) 4.0))
        (Variables|/Script/Engine.CharacterMovementComponent|SetMaxWalkSpeed (Variables|/Script/Engine.Character|GetCharacterMovement _asbp_split) 3e+02)
        (Variables|/Game/ActiveTowerDefense/Blueprints/BP_Enemy.BP_Enemy_C|SetAffix _asbp_split (Variables|Default|GetAffix))
        (Default|UpdateMaterial _asbp_split))
      (Actor|DestroyActor))))