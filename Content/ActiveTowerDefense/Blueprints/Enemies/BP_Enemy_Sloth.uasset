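; Sloth enemy Blueprint for the tower defense game that grows stronger the longer it is alive.
; A looping timer started on BeginPlay fires a growth event, which raises HP, scale, damage and walk speed until a small step cap is reached.
; The construction script tints the Sub component yellow-green through a dynamic material instance.
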(event Custom|growth
  (bind _charactermovement (Variables|Character|GetCharacterMovement))
  (if (<= (Variables|Default|GetgrowthStep) 2)
    (Variables|Default|SetHP (+ (Variables|Default|GetHP) 1e+01))
    (Transformation|SetActorScale3D (* (Transformation|GetActorScale3D) 1.25))
    (Variables|Default|SetDamage (+ (Variables|Default|GetDamage) 2.0))
    (Variables|/Script/Engine.CharacterMovementComponent|SetMaxWalkSpeed _charactermovement (+ (Variables|/Script/Engine.CharacterMovementComponent|GetMaxWalkSpeed _charactermovement) 5e+01))
    (Math|Integer|IncrementInt (Variables|Default|GetgrowthStep))))

(event EventBeginPlay
  (|CallParentFunction)
  (Utilities|Time|SetTimerbyEvent (delegate Custom|growth) 5.0 true))

(event Collision|EventActorBeginOverlap
  (params (OtherActor :type Actor%20Object%20Reference)))

(event EventTick
  (params (DeltaSeconds :type Float%20%28single-precision%29)))

(fn ConstructionScript
  (|CallParentFunction)
  (bind _returnvalue (Rendering|Material|CreateDynamicMaterialInstance (Variables|Default|Getsub) 0 0 "None" :!class /Script/Engine.PrimitiveComponent))
  (Rendering|Material|SetVectorParameterValue _returnvalue "color1" "(R=0.881586,G=1.000000,B=0.255081,A=1.000000)" :!class /Script/Engine.MaterialInstanceDynamic))