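; BP_Enemy is the tower defense enemy that walks to the actor returned by GetGamestate and explodes on it.
; After a short spawn delay, it loads stats and walk speed from TableData, then starts AIMoveTo.
; Arrival applies damage, spawns an explosion and destroys it; incoming damage reduces HP until Defeat destroys it.
; Armor is stored but unused, element material switching is disconnected, and gold worth is fixed.
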(event EventBeginPlay
  (Utilities|FlowControl|Delay 0.2)
  (Utilities|FlowControl|Sequence
    (:then_0
      (CallFunction|FromTableData (Variables|Default|GetTable%20Data)))
    (:then_1
      (bind _gamesstate (CallFunction|GetGamestate))
      (AI|AIMoveTo self "0, 0, 0" _gamesstate 5.0 false
        (:OnSuccess
          (CallFunction|ApplyDamage))))))

(event Game|Damage|EventAnyDamage
  (params (Damage :type Float%20%28single-precision%29) (DamageType :type Damage%20Type%20Object%20Reference) (InstigatedBy :type Controller%20Object%20Reference) (DamageCauser :type Actor%20Object%20Reference))
  (bind _output_get (Variables|Default|SetHP (- (Variables|Default|GetHP) Damage)))
  (if (<= _output_get 0.0)
    (CallFunction|Defeat)))

(fn ConstructionScript)

(fn Defeat
  (Actor|DestroyActor))

(fn UpdateMaterial)

(fn ApplyDamage
  (bind _gamesstate (CallFunction|GetGamestate))
  (Game|Damage|ApplyDamage _gamesstate (Variables|Default|GetDamage) 0 self "/Script/Engine.DamageType")
  (Effects|SpawnEmitteratLocation "/Game/StarterContent/Particles/P_Explosion.P_Explosion" (Transformation|GetWorldLocation (Variables|Character|GetMesh)))
  (Actor|DestroyActor))

(fn FromTableData
  (params (Enemy%20Data :type Struct%20Enemy%20Structure))
  (bind (_key _hp _damage _armor _movementspeed) (Utilities|Struct|BreakStruct_Enemy Enemy%20Data))
  (Variables|Default|SetAffix _key)
  (Variables|Default|SetHP _hp)
  (Variables|Default|SetDamage _damage)
  (Variables|Default|SetArmor _armor)
  (bind _output_get (Variables|/Script/Engine.CharacterMovementComponent|SetMaxWalkSpeed (Variables|Character|GetCharacterMovement) _movementspeed))
  (Development|PrintString (Utilities|String|ToString(Float) _output_get)))

(fn GetGoldWorth
  (return 1.0))