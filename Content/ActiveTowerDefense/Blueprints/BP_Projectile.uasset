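; Homing tower-defense projectile that flies at constant speed toward its target actor, destroying itself if the target becomes invalid.
; When its sphere overlaps that target, it applies damage, spawns an explosion effect and destroys itself.
; Base, nuke, elemental and AOE calculations are all called, but only the base result reaches the damage.
; The speed acceleration logic is disconnected and never runs.
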(event OnComponentBeginOverlap(Sphere)
  (params (OverlappedComponent :type Primitive%20Component%20Object%20Reference) (OtherActor :type Actor%20Object%20Reference) (OtherComp :type Primitive%20Component%20Object%20Reference) (OtherBodyIndex :type Integer) (bFromSweep :type Boolean) (SweepResult :type Hit%20Result%20Structure%20%28by%20ref%29))
  (if (== OtherActor (Variables|Default|GetProjectileTarget))
    (bind _basedamage (CallFunction|BaseDamageCalculation self))
    (bind _multiplier (CallFunction|NukeCalculation self))
    (bind _multiplier_2 (CallFunction|ElementalCalculation (Variables|Default|GetProjectileTarget) self))
    (bind _multiplier_3 (CallFunction|AOECalculation self))
    (Game|Damage|ApplyDamage (Variables|Default|GetProjectileTarget) _basedamage 0 0)
    (Effects|SpawnEmitteratLocation "/Game/StarterContent/Particles/P_Explosion.P_Explosion" (Transformation|GetWorldLocation (Variables|Default|GetStaticMesh)))
    (Actor|DestroyActor)))

(event EventTick
  (params (DeltaSeconds :type Float%20%28single-precision%29))
  (if (Utilities|IsValid (Variables|Default|GetProjectileTarget))
    (Transformation|SetActorLocation (Math|Interpolation|VInterptoConstant (Transformation|GetActorLocation) (Transformation|GetActorLocation (Variables|Default|GetProjectileTarget)) DeltaSeconds (Variables|Default|Getspeed)) false false)
    (else
      (Actor|DestroyActor))))

(fn ConstructionScript)