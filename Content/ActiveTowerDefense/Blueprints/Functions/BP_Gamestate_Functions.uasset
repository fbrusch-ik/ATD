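; Blueprint function library for a tower defense game, wrapping BP_Gamestate access to money, godmode and tower or buildable-area selection.
; Selection changes refresh area and tower materials, while enemy defeats award money by elite type.
; Damage helpers combine tower and ghost stats, scaling elemental and nuke multipliers through CT_Multipliers curves.
; BuyGhost charges after capacity checks but never reaches AddGhost; AOECalculation's return is unwired, and skill-widget functions are empty.
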(fn SetMoney
  (params (set :type Float%20%28single-precision%29))
  (bind _returnvalue (Actor|GetActorOfClass 0 "/Game/ActiveTowerDefense/Blueprints/BP_Gamestate.BP_Gamestate_C"))
  (bind _output_get (Variables|/Game/ActiveTowerDefense/Blueprints/BP_Gamestate.BP_Gamestate_C|Setmoney _returnvalue set))
  (return _output_get))

(fn GetMoney
  (bind _returnvalue (Actor|GetActorOfClass 0 "/Game/ActiveTowerDefense/Blueprints/BP_Gamestate.BP_Gamestate_C"))
  (return (Variables|/Game/ActiveTowerDefense/Blueprints/BP_Gamestate.BP_Gamestate_C|Getmoney _returnvalue)))

(fn Pay
  (params (cost :type Float%20%28single-precision%29))
  (bind _money (CallFunction|GetMoney))
  (if (>= _money cost)
    (bind _money_2 (CallFunction|GetMoney))
    (CallFunction|SetMoney (- _money_2 cost))
    (return true)
    (else
      (return false))))

(fn ToggleGodmode
  (bind _returnvalue (Actor|GetActorOfClass 0 "/Game/ActiveTowerDefense/Blueprints/BP_Gamestate.BP_Gamestate_C"))
  (Variables|/Game/ActiveTowerDefense/Blueprints/BP_Gamestate.BP_Gamestate_C|Setgodmode _returnvalue (not (Variables|/Game/ActiveTowerDefense/Blueprints/BP_Gamestate.BP_Gamestate_C|Getgodmode _returnvalue))))

(fn HasMoney
  (params (Money%20Required :type Float%20%28single-precision%29))
  (bind _money (CallFunction|GetMoney))
  (return (>= _money Money%20Required)))

(fn GetGamestate
  (bind _returnvalue (Actor|GetActorOfClass 0 "/Game/ActiveTowerDefense/Blueprints/BP_Gamestate.BP_Gamestate_C"))
  (return _returnvalue))

(fn BuyGhost
  (params (Type :type E_Ghosts%20Enum :default "NewEnumerator0"))
  (bind _newparam (CallFunction|GetGhostData Type))
  (LocalVariables|SetTotalCost (.cost _newparam))
  (LocalVariables|SetTotalSlots (.slots _newparam))
  (bind _selected_tower (CallFunction|HasSelectedTower))
  (Utilities|IsValid _selected_tower
    (:Is%20Valid
      (bind _hascapacity (Default|HasCapacity _selected_tower (LocalVariables|GetTotalSlots)))
      (if _hascapacity
        (bind _yes (CallFunction|HasMoney (LocalVariables|GetTotalCost)))
        (if _yes
          (CallFunction|Pay (LocalVariables|GetTotalCost)))))))

(fn GetSelectedTower
  (bind _returnvalue (Actor|GetActorOfClass 0 "/Game/ActiveTowerDefense/Blueprints/BP_Gamestate.BP_Gamestate_C"))
  (return (Variables|/Game/ActiveTowerDefense/Blueprints/BP_Gamestate.BP_Gamestate_C|GetselectedTower _returnvalue)))

(fn HasSelectedTower
  (bind _selectedtower (CallFunction|GetSelectedTower))
  (Utilities|IsValid _selectedtower
    (:Is%20Valid
      (return true _selectedtower))
    (:Is%20Not%20Valid
      (return false 0))))

(fn GetSelectedBuildableArea
  (bind _gamesstate (CallFunction|GetGamestate))
  (return (Variables|/Game/ActiveTowerDefense/Blueprints/BP_Gamestate.BP_Gamestate_C|GetselectedArea _gamesstate)))

(fn HasSelectedBuildableArea
  (bind _buildable_area (CallFunction|GetSelectedBuildableArea))
  (Utilities|IsValid _buildable_area
    (:Is%20Valid
      (return true _buildable_area))
    (:Is%20Not%20Valid
      (return false 0))))

(fn OpenSkillWidget)

(fn Select
  (params (Area :type BP%20Buildable%20Area%20Object%20Reference) (Tower :type BP%20Tower%20Object%20Reference))
  (bind _gamesstate (CallFunction|GetGamestate))
  (Variables|/Game/ActiveTowerDefense/Blueprints/BP_Gamestate.BP_Gamestate_C|SetselectedArea _gamesstate Area)
  (Variables|/Game/ActiveTowerDefense/Blueprints/BP_Gamestate.BP_Gamestate_C|SetselectedTower _gamesstate Tower)
  (CallFunction|UpdateAllMaterials)
  (Utilities|IsValid Tower))

(fn UpdateAllMaterials
  (bind _outactors (Actor|GetAllActorsOfClass 0 "/Game/ActiveTowerDefense/Blueprints/BP_BuildableArea.BP_BuildableArea_C"))
  (for _array_element _outactors
    (Default|UpdateMaterial _array_element)
    (bind _outactors_2 (Actor|GetAllActorsOfClass 0 "/Game/ActiveTowerDefense/Blueprints/BP_Tower.BP_Tower_C"))
    (for _array_element_2 _outactors_2
      (Default|UpdateMaterial _array_element_2))))

(fn CloseSkillWidget)

(fn ElementalCalculation
  (params (Damaged :type BP%20Enemy%20Object%20Reference) (Projectile :type BP%20Projectile%20Object%20Reference))
  (switch Utilities|FlowControl|Switch|SwitchonE_Elements (Variables|/Game/ActiveTowerDefense/Blueprints/BP_Enemy.BP_Enemy_C|Getenemy_type Damaged)
    (:NewEnumerator0
      (LocalVariables|Seteffective%20GT "NewEnumerator0"))
    (:NewEnumerator1
      (LocalVariables|Seteffective%20GT "NewEnumerator1"))
    (:NewEnumerator2
      (LocalVariables|Seteffective%20GT "NewEnumerator2"))
    (:NewEnumerator5
      (return 1.0)))
  (bind _count (Default|GetGhostCount (Variables|/Game/ActiveTowerDefense/Blueprints/BP_Projectile.BP_Projectile_C|GetTower Projectile) (LocalVariables|Geteffective%20GT)))
  (bind _outxy (DataTable|EvaluateCurveTableRow "/Game/ActiveTowerDefense/Data/CT_Multipliers.CT_Multipliers" "DamageMultipler" (Math|Conversions|ToFloat(Integer) _count))
    (:RowFound
      (return _outxy))))

(fn NukeCalculation
  (params (Projectile :type BP%20Projectile%20Object%20Reference))
  (bind _count (Default|GetGhostCount (Variables|/Game/ActiveTowerDefense/Blueprints/BP_Projectile.BP_Projectile_C|GetTower Projectile) "NewEnumerator4"))
  (bind _outxy (DataTable|EvaluateCurveTableRow "/Game/ActiveTowerDefense/Data/CT_Multipliers.CT_Multipliers" "DamageMultipler" (Math|Conversions|ToFloat(Integer) _count))
    (:RowFound
      (return _outxy))))

(fn AOECalculation
  (params (Projectile :type BP%20Projectile%20Object%20Reference))
  (bind _count (Default|GetGhostCount (Variables|/Game/ActiveTowerDefense/Blueprints/BP_Projectile.BP_Projectile_C|GetTower Projectile) "NewEnumerator3"))
  (bind _outxy (DataTable|EvaluateCurveTableRow "/Game/ActiveTowerDefense/Data/CT_Multipliers.CT_Multipliers" "AOEMultiplier" (Math|Conversions|ToFloat(Integer) _count))))

(fn EnemyDefeated
  (params (Defeated :type BP%20Enemy%20Object%20Reference))
  (CallFunction|GetGamestate)
  (bind _money (CallFunction|GetMoney))
  (switch Utilities|FlowControl|Switch|SwitchonE_Enemies (Variables|/Game/ActiveTowerDefense/Blueprints/BP_Enemy.BP_Enemy_C|Getelite_%20type Defeated)
    (:NewEnumerator0
      (LocalVariables|Setearned 1.0))
    (:NewEnumerator1
      (bind _asbp_split (Utilities|Casting|CastToBP_Split Defeated))
      (if (Variables|/Game/ActiveTowerDefense/Blueprints/BP_Split.BP_Split_C|Getchild _asbp_split)
        (LocalVariables|Setearned 0.0)
        (else
          (LocalVariables|Setearned 3.0))))
    (:NewEnumerator2
      (LocalVariables|Setearned 3.0))
    (:NewEnumerator3
      (LocalVariables|Setearned 3.0)))
  (CallFunction|SetMoney (+ _money (LocalVariables|Getearned)))
  (Default|DefeatEnemy Defeated))

(fn BaseDamageCalculation
  (params (Projectile :type BP%20Projectile%20Object%20Reference))
  (bind _tower (Variables|/Game/ActiveTowerDefense/Blueprints/BP_Projectile.BP_Projectile_C|GetTower Projectile))
  (bind _damage (Default|GetTotalGhostDamage _tower))
  (return (+ _damage (.basedamage (Variables|/Game/ActiveTowerDefense/Blueprints/BP_Tower.BP_Tower_C|GetTableData _tower)))))