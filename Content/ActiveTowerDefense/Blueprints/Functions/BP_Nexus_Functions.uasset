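; Function library for the tower defense game that gives shared access to the state held on the BP_Nexus actor, looked up by class on each call.
; It gets and sets Money, deducts a cost only when affordable, and toggles Godmode.
; Mount resets the previous tower's material, stores and highlights the new tower in yellow, and recreates the BP_TowerSkill widget.
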(fn SetMoney
  (params (set :type Float%20%28single-precision%29))
  (bind _returnvalue (Actor|GetActorOfClass 0 "/Game/ActiveTowerDefense/Blueprints/BP_Nexus.BP_Nexus_C"))
  (bind _output_get (Variables|/Game/ActiveTowerDefense/Blueprints/BP_Nexus.BP_Nexus_C|Setmoney _returnvalue set))
  (return _output_get))

(fn GetMoney
  (bind _returnvalue (Actor|GetActorOfClass 0 "/Game/ActiveTowerDefense/Blueprints/BP_Nexus.BP_Nexus_C"))
  (return (Variables|/Game/ActiveTowerDefense/Blueprints/BP_Nexus.BP_Nexus_C|Getmoney _returnvalue)))

(fn Pay
  (params (cost :type Float%20%28single-precision%29))
  (bind _money (CallFunction|GetMoney))
  (if (>= _money cost)
    (bind _money_2 (CallFunction|GetMoney))
    (CallFunction|SetMoney (- _money_2 cost))
    (return true)
    (else
      (return false))))

(fn Mount
  (params (mounted_tower :type BP%20Tower%20Object%20Reference))
  (Utilities|FlowControl|Sequence
    (:then_0
      (bind _returnvalue (Actor|GetActorOfClass 0 "/Game/ActiveTowerDefense/Blueprints/BP_Nexus.BP_Nexus_C"))
      (if (Utilities|IsValid (Variables|/Game/ActiveTowerDefense/Blueprints/BP_Nexus.BP_Nexus_C|GetmountedTower _returnvalue))
        (Default|ResetMaterial (Variables|/Game/ActiveTowerDefense/Blueprints/BP_Nexus.BP_Nexus_C|GetmountedTower _returnvalue))))
    (:then_1
      (bind _returnvalue_2 (Actor|GetActorOfClass 0 "/Game/ActiveTowerDefense/Blueprints/BP_Nexus.BP_Nexus_C"))
      (Variables|/Game/ActiveTowerDefense/Blueprints/BP_Nexus.BP_Nexus_C|SetmountedTower _returnvalue_2 mounted_tower)
      (bind _foundwidgets (Widget|GetAllWidgetsOfClass 0 "/Game/ActiveTowerDefense/Blueprints/UI/BP_TowerSkill.BP_TowerSkill_C"))
      (for _array_element _foundwidgets
        (Widget|RemovefromParent _array_element))
      (bind _returnvalue_3 (UserInterface|CreateWidget "/Game/ActiveTowerDefense/Blueprints/UI/BP_TowerSkill.BP_TowerSkill_C"))
      (UserInterface|Viewport|AddtoViewport _returnvalue_3 0))
    (:then_2
      (Rendering|Material|SetMaterial (Variables|/Game/ActiveTowerDefense/Blueprints/BP_Tower.BP_Tower_C|GetStaticMesh mounted_tower) 0 "/Game/ActiveTowerDefense/Materials/M_Element_yellow.M_Element_Yellow"))))

(fn ToggleGodmode
  (bind _returnvalue (Actor|GetActorOfClass 0 "/Game/ActiveTowerDefense/Blueprints/BP_Nexus.BP_Nexus_C"))
  (Variables|/Game/ActiveTowerDefense/Blueprints/BP_Nexus.BP_Nexus_C|Setgodmode _returnvalue (not (Variables|/Game/ActiveTowerDefense/Blueprints/BP_Nexus.BP_Nexus_C|Getgodmode _returnvalue))))