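; Selectable component for the tower defense game that handles mouse hover and click selection on its owning actor.
; On BeginPlay it binds to the owner's click and cursor-over events, tracks hover, and passes itself to Select when clicked.
; OnSelect and OnDeselect set the selected state.
; Each state change writes the mesh's custom depth stencil value to distinguish selected, hovered and idle, with selection taking priority.
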(event Custom|Clicked
  (params (TouchedActor :type Actor%20Object%20Reference) (ButtonPressed :type Key%20Structure :default "None"))
  (CallFunction|Select self))

(event Custom|Begin%20Hover
  (params (TouchedActor :type Actor%20Object%20Reference))
  (Variables|Default|SetHovered true)
  (CallFunction|UpdateBorder))

(event Custom|End%20Hover
  (params (TouchedActor :type Actor%20Object%20Reference))
  (Variables|Default|SetHovered false)
  (CallFunction|UpdateBorder))

(event EventBeginPlay
  (bind _returnvalue (Components|GetOwner))
  (EventDispatchers|BindEventtoOnClicked _returnvalue (delegate Custom|Clicked))
  (EventDispatchers|BindEventtoOnBeginCursorOver _returnvalue (delegate Custom|Begin%20Hover))
  (EventDispatchers|BindEventtoOnEndCursorOver _returnvalue (delegate Custom|End%20Hover)))

(event EventTick
  (params (DeltaSeconds :type Float%20%28single-precision%29)))

(fn OnSelect
  (Variables|Default|SetSelected true)
  (CallFunction|UpdateBorder))

(fn OnDeselect
  (Variables|Default|SetSelected false)
  (CallFunction|UpdateBorder))

(fn UpdateBorder
  (bind _mesh (Variables|Default|GetMesh))
  (if (Variables|Default|GetSelected)
    (Rendering|SetCustomDepthStencilValue _mesh 253)
    (elif (Variables|Default|GetHovered)
      (Rendering|SetCustomDepthStencilValue _mesh 252)
      (else
        (Rendering|SetCustomDepthStencilValue _mesh 0)))))