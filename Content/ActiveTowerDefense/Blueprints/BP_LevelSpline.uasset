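; BP_LevelSpline is an actor that lays a static mesh along an editable spline, in the Active Tower Defense game folder.
; Its construction script divides the spline length by a Distance variable and adds one spline mesh component per segment.
; Each segment takes local-space positions and tangents from the spline, with tangent lengths clamped to Distance to match segment length.
; The event graph has no active logic.
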(event EventBeginPlay)

(event Collision|EventActorBeginOverlap
  (params (OtherActor :type Actor%20Object%20Reference)))

(event EventTick
  (params (DeltaSeconds :type Float%20%28single-precision%29)))

(fn ConstructionScript
  (bind _spline (Variables|Default|GetSpline))
  (bind _distance (Variables|Default|GetDistance))
  (for _index (range 0 (.ReturnValue (Math|Float|Division(WholeandRemainder) (Spline|GetSplineLength _spline) (Variables|Default|GetDistance))))
    (bind _returnvalue (AddComponent|AddSplineMeshComponent false))
    (Components|StaticMesh|SetStaticMesh _returnvalue (Variables|Default|GetstaticMesh))
    (SplineMesh|SetStartandEnd _returnvalue (Spline|GetLocationatDistanceAlongSpline _spline (* _index _distance) "Local") (Math|Vector|ClampVectorSize (Spline|GetTangentatDistanceAlongSpline _spline (* _index _distance) "Local") _distance _distance) (Spline|GetLocationatDistanceAlongSpline _spline (+ (* _index _distance) _distance) "Local") (Math|Vector|ClampVectorSize (Spline|GetTangentatDistanceAlongSpline _spline (+ (* _index _distance) _distance) "Local") _distance _distance) true :!class /Script/Engine.SplineMeshComponent)))