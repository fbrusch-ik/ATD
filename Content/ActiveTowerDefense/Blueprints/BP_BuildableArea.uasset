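; BP_BuildableArea is a clickable build spot for towers in a tower defense game.
; Its static mesh swaps materials for default, hover, selected and disabled feedback, returning to the hover material on release.
; Clicking while Empty is true removes any existing BP_TowerBuilder widgets, then opens a new one with this area passed as BuildArea.
; Clicking an occupied area only shows the disabled material.
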(event OnBeginCursorOver(StaticMesh)
  (params (TouchedComponent :type Primitive%20Component%20Object%20Reference))
  (Rendering|Material|SetMaterial (Variables|Default|GetStaticMesh) 0 "/Game/ActiveTowerDefense/Materials/M_BuildArea_MouseOver.M_BuildArea_MouseOver"))

(event OnEndCursorOver(StaticMesh)
  (params (TouchedComponent :type Primitive%20Component%20Object%20Reference))
  (Rendering|Material|SetMaterial (Variables|Default|GetStaticMesh) 0 "/Game/ActiveTowerDefense/Materials/M_BuildArea_Default.M_BuildArea_Default"))

(event OnClicked(StaticMesh)
  (params (TouchedComponent :type Primitive%20Component%20Object%20Reference) (ButtonPressed :type Key%20Structure :default "None"))
  (bind _staticmesh (Variables|Default|GetStaticMesh))
  (if (Variables|Default|GetEmpty)
    (Rendering|Material|SetMaterial _staticmesh 0 "/Game/ActiveTowerDefense/Materials/M_BuildArea_Selected.M_BuildArea_Selected")
    (bind _foundwidgets (Widget|GetAllWidgetsOfClass "/Game/ActiveTowerDefense/Blueprints/UI/BP_TowerBuilder.BP_TowerBuilder_C" false))
    (for _array_element _foundwidgets
      (Widget|RemovefromParent _array_element))
    (bind _returnvalue (UserInterface|CreateWidget "/Game/ActiveTowerDefense/Blueprints/UI/BP_TowerBuilder.BP_TowerBuilder_C"))
    (Variables|/Game/ActiveTowerDefense/Blueprints/UI/BP_TowerBuilder.BP_TowerBuilder_C|SetBuildArea _returnvalue self)
    (UserInterface|Viewport|AddtoViewport _returnvalue 0)
    (else
      (Rendering|Material|SetMaterial _staticmesh 0 "/Game/ActiveTowerDefense/Materials/M_BuildArea_Disabled.M_BuildArea_Disabled"))))

(event OnReleased(StaticMesh)
  (params (TouchedComponent :type Primitive%20Component%20Object%20Reference) (ButtonReleased :type Key%20Structure :default "None"))
  (Rendering|Material|SetMaterial (Variables|Default|GetStaticMesh) 0 "/Game/ActiveTowerDefense/Materials/M_BuildArea_MouseOver.M_BuildArea_MouseOver"))

(fn ConstructionScript)