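; Unit manager actor that shows a placement preview following the mouse cursor in the tower defense game.
; StartAction enables build mode, stores the supplied data and applies its static mesh, skeletal mesh and scale to the placeholders.
; While building, Tick teleports the root to the Visibility cursor hit, offset by placeholder bounds, with height set from the bounds' sphere radius.
; Overlap events tint the sphere translucent orange or blue.
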(event EventBeginPlay)

(event EventTick
  (params (DeltaSeconds :type Float%20%28single-precision%29))
  (bind _placeholder (Variables|Default|GetPlaceholder))
  (bind (_origin _boxextent _sphereradius) (Collision|GetComponentBounds _placeholder))
  (if (Variables|Default|GetIsBuilding)
    (bind _location (CallFunction|GetMouseWorldLocation))
    (Transformation|SetWorldLocation (Variables|Default|GetDefaultSceneRoot) (Math|Vector|MakeVector (.x (+ (Math|Vector|MakeVector (/ (.x _boxextent) 2.0) (/ (.y _boxextent) 2.0) (.z _boxextent)) _location)) (.y (+ (Math|Vector|MakeVector (/ (.x _boxextent) 2.0) (/ (.y _boxextent) 2.0) (.z _boxextent)) _location)) _sphereradius) false true)))

(event Collision|EventActorBeginOverlap
  (params (OtherActor :type Actor%20Object%20Reference))
  (Rendering|Material|SetMaterial (Variables|Default|GetSphere) 0 "/Game/ActiveTowerDefense/Materials/M_TranslucentOrange.M_TranslucentOrange"))

(event Collision|EventActorEndOverlap
  (params (OtherActor :type Actor%20Object%20Reference))
  (Rendering|Material|SetMaterial (Variables|Default|GetSphere) 0 "/Game/ActiveTowerDefense/Materials/M_TranslucentBlue.M_TranslucentBlue"))

(fn ConstructionScript)

(fn StartAction
  (params (Data :type Struct%20Unit%20Action%20Structure))
  (Variables|Default|SetIsBuilding true)
  (bind _output_get (Variables|Default|SetCurrentData Data))
  (Components|StaticMesh|SetStaticMesh (Variables|Default|GetPlaceholder) (.placeholdermesh _output_get))
  (Physics|SetSimulatePhysics (Variables|Default|GetPlaceholder) true)
  (Class|SkinnedMeshComponent|SetSkeletalMesh (Variables|Default|GetPlaceholderSkeletal) (.placeholderskeletal _output_get) true)
  (Transformation|SetWorldScale3D (Variables|Default|GetPlaceholder) (Math|Conversions|ToVector(Float) (.meshscale _output_get))))

(fn GetMouseWorldLocation
  (bind _returnvalue (Game|GetPlayerController 0))
  (bind _hitresult (Game|Player|GetHitResultUnderCursorbyChannel _returnvalue "TraceTypeQuery1" true))
  (return (.location _hitresult) (.hitactor _hitresult)))