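; Tower building for a tower defense game that holds Ghosts up to an upgradeable capacity and auto-fires at nearby enemies.
; Tick runs a timed volley at random enemies in its sphere, with shot count read from a curve by the count of one Ghost type.
; Hover sets a stencil highlight, clicking Ghost1 selects the tower, and UpdateMaterial shows selection or tints by Ghost mix.
; Upgrades reveal higher-level meshes.
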(event OnClicked(Ghost1)
  (params (TouchedComponent :type Primitive%20Component%20Object%20Reference) (ButtonPressed :type Key%20Structure :default "None"))
  (CallFunction|Select 0 self))

(event EventBeginPlay)

(event MouseInput|EventActorBeginCursorOver
  (Rendering|SetCustomDepthStencilValue (Variables|Default|Gethouse) 252))

(event EventTick
  (params (DeltaSeconds :type Float%20%28single-precision%29))
  (Utilities|FlowControl|Sequence
    (:then_1
      (CallFunction|Autoshoot))))

(event MouseInput|EventActorEndCursorOver
  (Rendering|SetCustomDepthStencilValue (Variables|Default|Gethouse) 0))

(fn ConstructionScript
  (Variables|Default|Setcapacity (.startingcapacity (Variables|Default|GetTableData))))

(fn AddGhost
  (params (Ghost :type BP%20Ghost%20Object%20Reference))
  (bind _ghosts (Variables|Default|GetGhosts))
  (if (< (Utilities|Array|Length _ghosts) (Variables|Default|Getcapacity))
    (Utilities|Array|Add _ghosts Ghost)
    (return true)
    (else
      (return false))))

(fn HasCapacity
  (params (Slots%20Required :type Integer))
  (bind _ghost_count (CallFunction|TotalGhostCount))
  (return (<= (+ _ghost_count Slots%20Required) (Variables|Default|Getcapacity))))

(fn TotalGhostCount
  (return (Utilities|Array|Length (Variables|Default|GetGhosts))))

(fn UpgradeTower
  (bind _output_get (Variables|Default|Setcapacity (+ (Variables|Default|Getcapacity) 3)))
  (if (> _output_get 3)
    (Rendering|SetVisibility (Variables|Default|Getlevel2) true false)
    (if (> _output_get 6)
      (Rendering|SetVisibility (Variables|Default|Getlevel3) true false))))

(fn UpdateMaterial
  (bind _isselected (CallFunction|IsSelected))
  (if _isselected
    (Rendering|Material|SetMaterial (Variables|Default|Gethouse) 0 "/Game/ActiveTowerDefense/Materials/M_BuildArea_Selected.M_BuildArea_Selected")
    (bind _returnvalue (Rendering|Material|CreateDynamicMaterialInstance (Variables|Default|Getsub) 0 0 "None" :!class /Script/Engine.PrimitiveComponent))
    (Rendering|Material|SetVectorParameterValue _returnvalue "color1" "(R=1.000000,G=0.564711,B=0.026241,A=1.000000)" :!class /Script/Engine.MaterialInstanceDynamic)
    (bind _ghost_count (CallFunction|TotalGhostCount))
    (Effects|Components|ParticleSystem|SetFloatParameter (Variables|Default|Getsub) "rate" (Math|Conversions|ToFloat(Integer) _ghost_count))
    (else
      (Rendering|Material|SetMaterial (Variables|Default|Gethouse) 0 "/Game/StarterContent/Materials/M_Concrete_Grime.M_Concrete_Grime")
      (bind _returnvalue_2 (Rendering|Material|CreateDynamicMaterialInstance (Variables|Default|Getsub) 0 0 "None" :!class /Script/Engine.PrimitiveComponent))
      (bind _count (CallFunction|GetGhostCount "NewEnumerator0"))
      (bind _count_2 (CallFunction|GetGhostCount "NewEnumerator2"))
      (bind _count_3 (CallFunction|GetGhostCount "NewEnumerator1"))
      (bind _ghost_count_2 (CallFunction|TotalGhostCount))
      (Effects|Components|ParticleSystem|SetFloatParameter (Variables|Default|Getsub) "rate" (Math|Conversions|ToFloat(Integer) _ghost_count_2))
      (Rendering|Material|SetVectorParameterValue _returnvalue_2 "color1" (Utilities|Struct|MakeLinearColor (/ (Math|Conversions|ToFloat(Integer) _count) 3.0) (/ (Math|Conversions|ToFloat(Integer) _count_2) 3.0) (/ (Math|Conversions|ToFloat(Integer) _count_3) 3.0) 0.0) :!class /Script/Engine.MaterialInstanceDynamic))))

(fn IsSelected
  (bind _gamesstate (CallFunction|GetGamestate))
  (return (== (Variables|/Game/ActiveTowerDefense/Blueprints/BP_Gamestate.BP_Gamestate_C|GetselectedTower _gamesstate) self)))

(fn GetGhostCount
  (params (Type :type E_Ghosts%20Enum :default "NewEnumerator0"))
  (for _array_element (Variables|Default|GetGhosts)
    (if (== Type (.key (Variables|/Game/ActiveTowerDefense/Blueprints/Ghosts/BP_Ghost.BP_Ghost_C|GetTableData _array_element)))
      (Math|Integer|IncrementInt (LocalVariables|Getakku))))
  (return (LocalVariables|Getakku)))

(fn GetRandomEnemy
  (bind _overlappingactors (Collision|GetOverlappingActors "/Game/ActiveTowerDefense/Blueprints/Enemies/BP_Enemy.BP_Enemy_C" :!class /Script/Engine.Actor))
  (bind _asbp_enemy (Utilities|Casting|CastToBP_Enemy (Utilities|Array|Get(acopy) _overlappingactors (Math|Random|RandomIntegerinRange 0 (Utilities|Array|Length _overlappingactors)))))
  (return _asbp_enemy))

(fn Shoot
  (params (Projectile%20Target :type BP%20Enemy%20Object%20Reference))
  (Game|SpawnActorfromClass "/Game/ActiveTowerDefense/Blueprints/BP_Projectile.BP_Projectile_C" (Math|Conversions|ToTransform(Vector) (Transformation|GetWorldLocation (Utilities|Select :Index (Math|Random|RandomInteger 3) :Option%200 (Variables|Default|GetGhost2) :Option%201 (Variables|Default|GetGhost3) :Option%202 (Variables|Default|GetGhost4)))) "AlwaysSpawn" 0 Projectile%20Target self 0))

(fn GetTotalGhostDamage
  (for _array_element (Variables|Default|GetGhosts)
    (LocalVariables|SetDamage%20Akku (+ (.basedamage (Variables|/Game/ActiveTowerDefense/Blueprints/Ghosts/BP_Ghost.BP_Ghost_C|GetTableData _array_element)) (LocalVariables|GetDamage%20Akku))))
  (return (LocalVariables|GetDamage%20Akku)))

(fn GetRandomEnemies
  (params (Count :type Integer) (Allow%20Duplicates :type Boolean))
  (bind _output_get (LocalVariables|SetOverlapping (Collision|GetOverlappingActors (Variables|Default|GetSphere) "/Game/ActiveTowerDefense/Blueprints/Enemies/BP_Enemy.BP_Enemy_C" :!class /Script/Engine.PrimitiveComponent)))
  (if (> (Utilities|Array|Length _output_get) 0)
    (Utilities|Array|Shuffle (LocalVariables|GetOverlapping) :!label _label)
    (bind _array_element (Utilities|Array|ForEachLoopwithBreak (LocalVariables|GetOverlapping))
      (:LoopBody
        (if (== (Utilities|Array|Length (LocalVariables|GetEnemies)) Count)
          (return (LocalVariables|GetEnemies))
          (else
            (bind _asbp_enemy (Utilities|Casting|CastToBP_Enemy _array_element))
            (Utilities|Array|Add (LocalVariables|GetEnemies) _asbp_enemy))))
      (:Completed
        (if Allow%20Duplicates
          (goto _label)
          (else
            (return (LocalVariables|GetEnemies))))))
    (else
      (return (LocalVariables|GetEnemies)))))

(fn Autoshoot
  (bind _returnvalue (Utilities|Time|GetGameTimeinSeconds))
  (Math|Float|CompareFloat (Variables|Default|GetfireTimer) _returnvalue
    (:<
      (bind _count (CallFunction|GetGhostCount "NewEnumerator3"))
      (bind _outxy (DataTable|EvaluateCurveTableRow "/Game/ActiveTowerDefense/Data/CT_Multipliers.CT_Multipliers" "AOEShots" (Math|Conversions|ToFloat(Integer) _count))
        (:RowFound
          (bind _newparam (CallFunction|GetRandomEnemies (Math|Float|Truncate _outxy) true))
          (for _array_element _newparam
            (CallFunction|Shoot _array_element))
          (Variables|Default|SetfireTimer (+ _returnvalue (.firingrate (Variables|Default|GetTableData)))))))))

(fn UpdateInventory)