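; BP_BuildableArea is a clickable build spot for placing towers in a tower defense game.
; Cursor hover updates its mesh material to show default, hovered, selected or disabled, with selection read from the GameState's SelectedArea.
; Releasing a click on the mesh selects the area.
; BuildTower spawns a BP_Tower at the area's transform, marks it occupied, selects the new tower and destroys the area.
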(event OnBeginCursorOver(StaticMesh)
  (params (TouchedComponent :type Primitive%20Component%20Object%20Reference))
  (Variables|Default|SetmouseOver true)
  (CallFunction|UpdateMaterial))

(event OnEndCursorOver(StaticMesh)
  (params (TouchedComponent :type Primitive%20Component%20Object%20Reference))
  (Variables|Default|SetmouseOver false)
  (CallFunction|UpdateMaterial))

(event OnReleased(StaticMesh)
  (params (TouchedComponent :type Primitive%20Component%20Object%20Reference) (ButtonReleased :type Key%20Structure))
  (CallFunction|Select self))

(fn ConstructionScript)

(fn IsSelected
  (bind _gamesstate (CallFunction|GetGamestate))
  (return (== (Variables|/Game/ActiveTowerDefense/Blueprints/BP_Gamestate.BP_Gamestate_C|GetselectedArea _gamesstate) self)))

(fn UpdateMaterial
  (if (Variables|Default|GetEmpty)
    (bind _isselected (CallFunction|IsSelected))
    (if _isselected
      (Rendering|Material|SetMaterial (Variables|Default|GetStaticMesh) 0 "/Game/ActiveTowerDefense/Materials/M_BuildArea_Selected.M_BuildArea_Selected")
      (elif (Variables|Default|GetmouseOver)
        (Rendering|Material|SetMaterial (Variables|Default|GetStaticMesh) 0 "/Game/ActiveTowerDefense/Materials/M_BuildArea_MouseOver.M_BuildArea_MouseOver")
        (else
          (Rendering|Material|SetMaterial (Variables|Default|GetStaticMesh) 0 "/Game/ActiveTowerDefense/Materials/M_BuildArea_Default.M_BuildArea_Default"))))
    (else
      (Rendering|Material|SetMaterial (Variables|Default|GetStaticMesh) 0 "/Game/ActiveTowerDefense/Materials/M_BuildArea_Disabled.M_BuildArea_Disabled"))))

(fn BuildTower
  (bind _returnvalue (Game|SpawnActorfromClass :Class "/Game/ActiveTowerDefense/Blueprints/Buildings/BP_Tower.BP_Tower_C" :SpawnTransform (Transformation|GetActorTransform) :CollisionHandlingOverride "Undefined" :Instigator 0))
  (Variables|Default|SetEmpty false)
  (CallFunction|Select 0 _returnvalue)
  (Actor|DestroyActor))