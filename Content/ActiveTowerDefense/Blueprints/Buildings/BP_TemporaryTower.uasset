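; BP_TemporaryTower is a placement preview for a tower that follows the mouse's world location every tick.
; Each tick its Box checks for overlaps with the level spline or existing towers.
; A helper swaps every material on the Tower component to translucent orange when overlapping and translucent blue otherwise.
; The construction script applies a default build-area material, and the actor only gives visual feedback, with no placement logic.
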(event EventBeginPlay)

(event Collision|EventActorBeginOverlap
  (params (OtherActor :type Actor%20Object%20Reference)))

(event EventTick
  (params (DeltaSeconds :type Float%20%28single-precision%29))
  (if true
    (bind _location (CallFunction|GetMouseWorldLocation))
    (Transformation|SetWorldLocation (Variables|Default|GetSceneRoot) (Math|Vector|MakeVector (.x _location) (.y _location) (.z _location)) false true)
    (bind _overlapping (CallFunction|IsOverlapping "/Game/ActiveTowerDefense/Blueprints/BP_LevelSpline.BP_LevelSpline_C"))
    (bind _overlapping_2 (CallFunction|IsOverlapping "/Game/ActiveTowerDefense/Blueprints/Buildings/BP_Tower.BP_Tower_C"))
    (if (or _overlapping_2 _overlapping)
      (CallFunction|SetAllMaterials "/Game/ActiveTowerDefense/Materials/M_TranslucentOrange.M_TranslucentOrange")
      (else
        (CallFunction|SetAllMaterials "/Game/ActiveTowerDefense/Materials/M_TranslucentBlue.M_TranslucentBlue")))))

(fn ConstructionScript
  (CallFunction|SetAllMaterials "/Game/ActiveTowerDefense/Materials/M_BuildArea_Default.M_BuildArea_Default"))

(fn SetAllMaterials
  (params (Material :type Material%20Object%20Reference))
  (for (_ _array_index) (Rendering|Material|GetMaterials (Variables|Default|GetTower))
    (Rendering|Material|SetMaterial (Variables|Default|GetTower) _array_index Material)))

(fn IsOverlapping
  (params (Filter :type Actor%20Class%20Reference))
  (return (> (Utilities|Array|Length (Collision|GetOverlappingActors (Variables|Default|GetBox) Filter :!class /Script/Engine.PrimitiveComponent)) 0)))