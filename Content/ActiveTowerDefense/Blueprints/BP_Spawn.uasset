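; BP_Spawn is a spawn point for enemies in the active tower defense game.
; Its spawn_enemy event spawns a BP_Enemy with AI at the actor's own location.
; It then picks one of the green, red or blue element materials at random and applies it to the first material slot of the enemy's mesh.
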(event Custom|spawn_enemy
  (bind _returnvalue (AI|SpawnAIFromClass "/Game/ActiveTowerDefense/Blueprints/BP_Enemy.BP_Enemy_C" 0 (Transformation|GetActorLocation) "0, 0, 0" false 0))
  (bind _asbp_enemy (Utilities|Casting|CastToBP_Enemy _returnvalue))
  (Utilities|FlowControl|Sequence
    (:then_0
      (switch int (Math|Random|RandomInteger 3)
        (:0
          (Variables|Default|SetrandomMaterial "/Game/ActiveTowerDefense/Materials/M_Element_Green.M_Element_Green"))
        (:1
          (Variables|Default|SetrandomMaterial "/Game/ActiveTowerDefense/Materials/M_Element_Red.M_Element_Red"))
        (:2
          (Variables|Default|SetrandomMaterial "/Game/ActiveTowerDefense/Materials/M_Element_Blue.M_Element_Blue"))))
    (:then_1
      (Rendering|Material|SetMaterial (Variables|/Script/Engine.Character|GetMesh _asbp_enemy) 0 (Variables|Default|GetrandomMaterial)))))

(fn ConstructionScript)