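; Clickable tower defense tower that fires BP_Projectile at overlapping enemies, passing its current material to each shot.
; Tick fires once FireTimer elapses, targeting one random overlapping actor, or every enemy during timed Multishot.
; It stores red, blue and green ghost counts with a separate capacity check, and upgrades raise capacity and reveal level components.
; Clicking selects the tower, and UpdateMaterial reflects whether it is the game state's SelectedTower.
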(event OnClicked(StaticMesh)
  (params (TouchedComponent :type Primitive%20Component%20Object%20Reference) (ButtonPressed :type Key%20Structure :default "None"))
  (CallFunction|Select 0 self))

(event EventTick
  (params (DeltaSeconds :type Float%20%28single-precision%29))
  (bind _overlappingactors (Collision|GetOverlappingActors 0 :!class /Script/Engine.Actor))
  (bind _returnvalue (Transformation|GetActorTransform))
  (bind _returnvalue_2 (Utilities|Time|GetGameTimeinSeconds))
  (Math|Float|CompareFloat (Variables|Default|GetfireTimer) _returnvalue_2
    (:<
      (if (Variables|Default|Getmultishot)
        (for _array_element _overlappingactors
          (bind _asbp_enemy (Utilities|Casting|CastToBP_Enemy _array_element))
          (bind _returnvalue_3 (Game|SpawnActorfromClass "/Game/ActiveTowerDefense/Blueprints/BP_Projectile.BP_Projectile_C" _returnvalue "AlwaysSpawn" 0 _asbp_enemy 0))
          (Rendering|Material|SetMaterial (Variables|/Game/ActiveTowerDefense/Blueprints/BP_Projectile.BP_Projectile_C|GetStaticMesh _returnvalue_3) 0 (Rendering|Material|GetMaterial (Variables|Default|GetStaticMesh) 0))
          (Variables|Default|SetfireTimer (+ _returnvalue_2 (Variables|Default|GetfiringRate))))
        (else
          (bind _asbp_enemy_2 (Utilities|Casting|CastToBP_Enemy (Utilities|Array|Get(acopy) _overlappingactors (Math|Random|RandomIntegerinRange 0 (Utilities|Array|Length _overlappingactors)))))
          (bind _returnvalue_4 (Game|SpawnActorfromClass "/Game/ActiveTowerDefense/Blueprints/BP_Projectile.BP_Projectile_C" _returnvalue "AlwaysSpawn" 0 _asbp_enemy_2 0))
          (Rendering|Material|SetMaterial (Variables|/Game/ActiveTowerDefense/Blueprints/BP_Projectile.BP_Projectile_C|GetStaticMesh _returnvalue_4) 0 (Rendering|Material|GetMaterial (Variables|Default|GetStaticMesh) 0))
          (Variables|Default|SetfireTimer (+ _returnvalue_2 (Variables|Default|GetfiringRate))))))))

(fn ConstructionScript)

(fn EnableMultishot
  (Variables|Default|Setmultishot true)
  (Utilities|Time|SetTimerbyFunctionName 0 "Disable Multishot" (Variables|Default|Getmultishot_timer)))

(fn DisableMultishot
  (Variables|Default|Setmultishot false))

(fn AddGhost
  (params (amount :type Integer) (type :type ghost_types%20Enum :default "NewEnumerator0"))
  (CallFunction|SetGhostInternal type amount)
  (return false))

(fn SetGhostInternal
  (params (Type :type ghost_types%20Enum :default "NewEnumerator0") (Amount :type Integer))
  (switch Utilities|FlowControl|Switch|Switchonghost_types Type
    (:NewEnumerator0
      (Variables|Default|Setred_count (+ (Variables|Default|Getred_count) Amount)))
    (:NewEnumerator1
      (Variables|Default|Setblue_count (+ (Variables|Default|Getblue_count) Amount)))
    (:NewEnumerator2
      (Variables|Default|Setgreen_count (+ (Variables|Default|Getgreen_count) Amount)))))

(fn HasCapacity
  (params (Slots%20Required :type Integer))
  (bind _ghost_count (CallFunction|TotalGhostCount))
  (return (<= (+ _ghost_count Slots%20Required) (Variables|Default|Getcapacity))))

(fn TotalGhostCount
  (return (+ (Variables|Default|Getred_count) (Variables|Default|Getgreen_count) (Variables|Default|Getblue_count))))

(fn UpgradeTower
  (bind _output_get (Variables|Default|Setcapacity (+ (Variables|Default|Getcapacity) 3)))
  (if (> _output_get 3)
    (Rendering|SetVisibility (Variables|Default|Getlevel2) true false)
    (if (> _output_get 6)
      (Rendering|SetVisibility (Variables|Default|Getlevel3) true false))))

(fn UpdateMaterial
  (bind _staticmesh (Variables|Default|GetStaticMesh))
  (bind _isselected (CallFunction|IsSelected))
  (if _isselected
    (Rendering|Material|SetMaterial _staticmesh 0 "/Game/ActiveTowerDefense/Materials/M_BuildArea_Selected.M_BuildArea_Selected")
    (else
      (Rendering|Material|SetMaterial _staticmesh 0 "/Game/StarterContent/Materials/M_Concrete_Grime.M_Concrete_Grime"))))

(fn IsSelected
  (bind _gamesstate (CallFunction|GetGamestate))
  (return (== (Variables|/Game/ActiveTowerDefense/Blueprints/BP_Gamestate.BP_Gamestate_C|GetselectedTower _gamesstate) self)))

(fn GetGhostCount
  (params (Type :type ghost_types%20Enum :default "NewEnumerator0"))
  (switch Utilities|FlowControl|Switch|Switchonghost_types Type
    (:NewEnumerator0
      (return (Variables|Default|Getred_count)))
    (:NewEnumerator1
      (return (Variables|Default|Getblue_count)))
    (:NewEnumerator2
      (return (Variables|Default|Getgreen_count)))))